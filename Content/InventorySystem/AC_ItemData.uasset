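; Item data component that makes its owning actor a pickup for the inventory system.
; On interaction, it adds its item ID and quantity to the character's inventory component.
; If that succeeds, it plays a pickup sound from DT_ItemTable, always read from the hardcoded "gold" row, and destroys the owner.
; It disables owner replication on BeginPlay, and its Look At function returns empty text.
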(event EventInteractwith
  (params (Character :type BP%20Ranger%20Object%20Reference))
  (bind _ac_inventorysystem (Variables|/Game/Gunslinger/Blueprints/Characters/BP_Ranger.BP_Ranger_C|GetAC_InventorySystem Character))
  (Utilities|IsValid _ac_inventorysystem
    (:Is%20Valid
      (bind _success (Default|AddtoInventory _ac_inventorysystem (.rowname (Variables|Default|GetItemID)) (Variables|Default|GetQuantity)))
      (if _success
        (bind _returnvalue (Utilities|GetDataTableRow "/Game/InventorySystem/DT_ItemTable.DT_ItemTable" "gold")
          (:then
            (Audio|PlaySound2D (.pickupsound _returnvalue) 1.0 1.0 0.0 0 0)
            (Actor|DestroyActor (Components|GetOwner))))))))

(event EventBeginPlay
  (Networking|SetReplicates (Components|GetOwner) false))

(fn Lookat
  (return ""))