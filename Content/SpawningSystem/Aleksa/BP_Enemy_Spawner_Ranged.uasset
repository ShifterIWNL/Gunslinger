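; Enemy spawner actor that creates ranged or melee enemies at its own transform while the player is nearby.
; Tick sets an in-range flag from the distance to the player pawn, and a looping timer started at BeginPlay calls Spawn Enemy.
; Each spawn randomly picks either enemy type with equal odds and plays a spawn sound.
; MaxEnemyCount counts spawns and is never decremented here, capping the total rather than living enemies.
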(event EventTick
  (params (DeltaSeconds :type Float%20%28single-precision%29))
  (if (< (Transformation|GetDistanceTo (Game|Player|GetPlayerPawn 0)) 1.2e+03)
    (Variables|Default|SetInSpawnRange true)
    (else
      (Variables|Default|SetInSpawnRange false))))

(event EventBeginPlay
  (Utilities|Time|SetTimerbyFunctionName 0 "Spawn Enemy" 5.0 true))

(fn ConstructionScript)

(fn SpawnEnemyRanged
  (Game|SpawnActorfromClass "/Game/Gunslinger/Blueprints/Characters/BP_EnemyRanged.BP_EnemyRanged_C" (Transformation|GetActorTransform self) "Undefined" "MultiplyWithRoot" 0 0.0 0)
  (Audio|PlaySoundatLocation "/Game/Gunslinger/Sounds/MapSounds/Enemy_Spawn.Enemy_Spawn" (Transformation|GetActorLocation self) "0, 0, 0" 1.0 1.0 0.0 0 0 0 0)
  (return))

(fn SpawnEnemy
  (if (and (< (Variables|Default|GetMax%20Enemy%20Count) 4) (Variables|Default|GetInSpawnRange))
    (if (Math|Random|RandomBoolwithWeight 0.5)
      (CallFunction|SpawnEnemyRanged)
      (else
        (CallFunction|SpawnEnemyMelee)))
    (Math|Integer|IncrementInt (Variables|Default|GetMax%20Enemy%20Count)
      (:%20%20
        (return)))))

(fn SpawnEnemyMelee
  (Game|SpawnActorfromClass "/Game/Gunslinger/Blueprints/Characters/BP_Enemy_Melee.BP_Enemy_Melee_C" (Transformation|GetActorTransform self) "Undefined" "MultiplyWithRoot" 0 0.0 0)
  (Audio|PlaySoundatLocation "/Game/Gunslinger/Sounds/MapSounds/Enemy_Spawn.Enemy_Spawn" (Transformation|GetActorLocation self) "0, 0, 0" 1.0 1.0 0.0 0 0 0 0)
  (return))