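; BP_Projectile_Grenade is a skeleton weapon projectile that explodes on impact and damages the BP_Ranger it hits.
; On sphere hit, it ignores BP_EnemyRanged actors, otherwise fires the impact callback, plays sound and pooled particles, then destroys itself.
; Damage is direct-hit only: the instigator's Ability System Component applies GE_Damage_Skeleton to the Ranger, with no radial check.
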(event OnComponentHit(Sphere)
  (params (HitComponent :type Primitive%20Component%20Object%20Reference) (OtherActor :type Actor%20Object%20Reference) (OtherComp :type Primitive%20Component%20Object%20Reference) (NormalImpulse :type Vector :default "0, 0, 0") (Hit :type Hit%20Result%20Structure%20%28by%20ref%29))
  (bind _returnvalue (Transformation|GetActorLocation))
  (bind _returnvalue_2 (Game|GetInstigator))
  (bind _returnvalue_3 (Ability|GetAbilitySystemComponent _returnvalue_2))
  (if (not (== (Utilities|GetClass OtherActor) "/Game/Gunslinger/Blueprints/Characters/BP_EnemyRanged.BP_EnemyRanged_C"))
    (Default|CallOnProjectileImpact OtherActor Hit)
    (Audio|SpawnSoundatLocation (Variables|Sounds|GetImpactSound) _returnvalue "0, 0, 0" 0.8 1.0 0.0 "/Game/Assets/MilitaryWeapSilver/Sound/Attenuation/Explosion_att.Explosion_att" 0)
    (Effects|SpawnEmitteratLocation (Variables|Effects|GetImpactEffect) _returnvalue "0, 0, 0" "0.400000,0.400000,0.400000" true "AutoRelease")
    (Actor|DestroyActor)
    (bind _asbp_ranger (Utilities|Casting|CastToBP_Ranger OtherActor))
    (GameplayEffects|ApplyGameplayEffectToTarget _returnvalue_3 "/Game/Gunslinger/Blueprints/Gameplay/Effects/GE_Damage_Skeleton.GE_Damage_Skeleton_C" (Variables|/Script/Gunslinger.GunslingerCharacter|GetAbilitySystemComponent _asbp_ranger) 0.0 (GameplayEffects|MakeEffectContext _returnvalue_3))))

(fn ConstructionScript
  (|CallParentFunction))