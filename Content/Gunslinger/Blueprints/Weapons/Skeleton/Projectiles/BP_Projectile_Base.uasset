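; BP_Projectile_Base is a projectile Blueprint, named as a base for weapon projectiles in Gunslinger.
; Its construction script copies the Speed variable into the ProjectileMovement component's initial speed.
; Logic for max speed, gravity scale and optional homing on a valid Target's root component is present but disconnected, so it never runs.
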(fn ConstructionScript
  (Variables|/Script/Engine.ProjectileMovementComponent|SetInitialSpeed (Variables|Default|GetProjectileMovement) (Variables|ProjectileSettings|GetSpeed)))