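; BP_EnemyBoss is the boss enemy, whose destruction triggers the player's victory.
; On Destroyed, it confirms the player pawn is a BP_Ranger, then creates and shows the WBP_VictoryScreen widget, switches input to UI only and pauses the game.
; The construction script only calls its parent, and nothing else is defined in these graphs.
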(event EventDestroyed
  (bind _returnvalue (Game|GetPlayerController 0))
  (bind _asbp_ranger (Utilities|Casting|CastToBP_Ranger (Game|Player|GetPlayerPawn 0)))
  (bind _returnvalue_2 (UserInterface|CreateWidget "/Game/Gunslinger/Blueprints/UI/HUD/WBP_VictoryScreen.WBP_VictoryScreen_C" _returnvalue))
  (Variables|/Script/UMG.Widget|SetVisibility _returnvalue_2 "Visible")
  (Input|SetInputModeUIOnly _returnvalue _returnvalue_2 "DoNotLock" false)
  (Game|SetGamePaused true)
  (UserInterface|Viewport|AddtoViewport _returnvalue_2 0))

(fn ConstructionScript
  (|CallParentFunction))