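; Ranged bomber enemy that throws grenades at the player.
; Attack plays a throw montage, reports attack end on completion or interruption, and on its notify spawns a grenade at HammerSocket.
; The grenade is aimed along a suggested ballistic toss toward the player, with launch speed scaled by distance.
; Overrides set walk speed per movement state and supply ideal attack and strafe ranges.
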(event EventAttack
  (bind _returnvalue (Game|GetPlayerCharacter 0))
  (bind _mesh (Variables|Character|GetMesh))
  (bind _returnvalue_2 (Transformation|GetSocketLocation _mesh "HammerSocket"))
  (bind _returnvalue_3 (Transformation|GetActorLocation _returnvalue))
  (bind _returnvalue_4 (- _returnvalue_3 _returnvalue_2))
  (bind _returnvalue_5 (Math|Vector|VectorLength _returnvalue_4))
  (bind _returnvalue_6 (* _returnvalue_5 1.5))
  (Animation|Montage|PlayMontage _mesh "/Game/Gunslinger/Animations/Skeleton/AM_Bomber_Attack_Throw.AM_Bomber_Attack_Throw"
    (:OnCompleted
      (Default|CallOnAttackEnd :!label _label))
    (:OnInterrupted
      (goto _label))
    (:OnNotifyBegin
      (bind _tossvelocity (Class|GameplayStatics|BlueprintSuggestProjectileVelocity _returnvalue_2 _returnvalue_3 _returnvalue_6 0.0 "DoNotTrace" 5.0 false false))
      (Game|SpawnActorfromClass "/Game/Gunslinger/Blueprints/Weapons/Skeleton/Projectiles/BP_Projectile_Grenade.BP_Projectile_Grenade_C" (Math|Transform|MakeTransform (.Location (Math|Transform|BreakTransform (Transformation|GetSocketTransform _mesh "HammerSocket" "RTS_World"))) (Math|Rotator|MakeRotfromX _tossvelocity)) "Undefined" "MultiplyWithRoot" 0 _returnvalue_6 0.0 0 false self))))

(fn ConstructionScript
  (|CallParentFunction))

(fn SetMovementSpeed
  (params (Speed :type E_MovementSpeed%20Enum :default "NewEnumerator0"))
  (bind _output_get (Variables|/Script/Engine.CharacterMovementComponent|SetMaxWalkSpeed (Variables|Character|GetCharacterMovement) (Utilities|Select :Index Speed :NewEnumerator0 0.0 :NewEnumerator1 1.3e+02 :NewEnumerator2 2.6e+02 :NewEnumerator3 3.4e+02)))
  (return _output_get))

(fn GetIdealRange
  (return 8e+02 8e+02))