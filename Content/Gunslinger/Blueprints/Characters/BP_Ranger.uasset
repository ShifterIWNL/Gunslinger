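; BP_Ranger is a playable gunslinger character built on the Gameplay Ability System.
; Enhanced Input drives movement, turn-in-place flags and pause, and activates jump, roll, shoot and reload abilities.
; BeginPlay applies initial attributes, creates HUD widgets and watches an attribute to trigger hurt feedback or a one-time death sequence.
; Trigger-volume overlaps switch footstep sounds, capsule hits can clear the airborne effect, and inventory component activation calls its local interact.
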(event OnComponentActivated(AC_InventorySystem)
  (params (Component :type Actor%20Component%20Object%20Reference) (bReset :type Boolean))
  (bind _asac_inventory_system (Utilities|Casting|CastToAC_InventorySystem Component))
  (Default|OnLocalInteract _asac_inventory_system))

(event OnComponentHit(CapsuleComponent)
  (params (HitComponent :type Primitive%20Component%20Object%20Reference) (OtherActor :type Actor%20Object%20Reference) (OtherComp :type Primitive%20Component%20Object%20Reference) (NormalImpulse :type Vector :default "0, 0, 0") (Hit :type Hit%20Result%20Structure%20%28by%20ref%29))
  (if (< (.Z (Math|Vector|BreakVector (Transformation|GetVelocity))) 1.0)
    (GameplayEffects|RemoveActiveGameplayEffectbySourceEffect (Variables|Default|GetAbilitySystemComponent) "/Game/Gunslinger/Blueprints/Gameplay/Effects/GE_IsAirborne.GE_IsAirborne_C" 0 -1)))

(event Input|EnhancedActionEvents|EnhancedInputActionIA_Reload
  (params (ActionValue :type Boolean) (ElapsedSeconds :type Float%20%28double-precision%29) (TriggeredSeconds :type Float%20%28double-precision%29) (InputAction :type Input%20Action%20Object%20Reference :default "/Game/Gunslinger/Input/IA_Reload.IA_Reload"))
  (Abilities|TryActivateAbilitybyClass (Variables|Default|GetAbilitySystemComponent) "/Game/Gunslinger/Blueprints/Gameplay/Abilities/GA_Reload.GA_Reload_C" true)
  (Default|CallReloaded))

(event Input|EnhancedActionEvents|EnhancedInputActionIA_Move
  (params (ActionValue :type Vector%202D%20Structure) (ElapsedSeconds :type Float%20%28double-precision%29) (TriggeredSeconds :type Float%20%28double-precision%29) (InputAction :type Input%20Action%20Object%20Reference :default "/Game/Gunslinger/Input/IA_Move.IA_Move"))
  (Variables|Default|SetMovement (Math|Vector2D|MakeVector2D (.x ActionValue) (.y ActionValue)))
  (Pawn|Input|AddMovementInput (Transformation|GetActorForwardVector) (.x ActionValue) false)
  (Pawn|Input|AddMovementInput (Transformation|GetActorRightVector) (.y ActionValue) false))

(event Input|EnhancedActionEvents|EnhancedInputActionIA_Shoot
  (params (ActionValue :type Boolean) (ElapsedSeconds :type Float%20%28double-precision%29) (TriggeredSeconds :type Float%20%28double-precision%29) (InputAction :type Input%20Action%20Object%20Reference :default "/Game/Gunslinger/Input/IA_Shoot.IA_Shoot"))
  (Abilities|TryActivateAbilitybyClass (Variables|Default|GetAbilitySystemComponent) "/Game/Gunslinger/Blueprints/Gameplay/Abilities/GA_Pistol_Shoot_Ranger.GA_Pistol_Shoot_Ranger_C" true)
  (Default|CallFiredShot))

(event Input|EnhancedActionEvents|EnhancedInputActionIA_Jump
  (params (ActionValue :type Boolean) (ElapsedSeconds :type Float%20%28double-precision%29) (TriggeredSeconds :type Float%20%28double-precision%29) (InputAction :type Input%20Action%20Object%20Reference :default "/Game/Gunslinger/Input/IA_Jump.IA_Jump"))
  (if (not (Variables|Default|GetRolling))
    (Abilities|TryActivateAbilitybyClass (Variables|Default|GetAbilitySystemComponent) "/Game/Gunslinger/Blueprints/Gameplay/Abilities/GA_Jump.GA_Jump_C" true)))

(event Input|EnhancedActionEvents|EnhancedInputActionIA_Roll
  (params (ActionValue :type Boolean) (ElapsedSeconds :type Float%20%28double-precision%29) (TriggeredSeconds :type Float%20%28double-precision%29) (InputAction :type Input%20Action%20Object%20Reference :default "/Game/Gunslinger/Input/IA_Roll.IA_Roll"))
  (:Triggered
    (if (and (not (AI|Components|NavMovement|IsFalling (Variables|Character|GetCharacterMovement))) (not (GameplayTags|HasMatchingGameplayTag (Variables|Default|GetAbilitySystemComponent) "(TagName=\"Roll.Cooldown\")")))
      (Variables|Default|SetRolling true)
      (Abilities|TryActivateAbilitybyClass (Variables|Default|GetAbilitySystemComponent) "/Game/Gunslinger/Blueprints/Gameplay/Abilities/GA_Roll.GA_Roll_C" true)))
  (:Started
    (Utilities|FlowControl|Delay 0.8)
    (Variables|Default|SetRolling false)))

(event Input|EnhancedActionEvents|EnhancedInputActionIA_Look
  (params (ActionValue :type Vector%202D%20Structure) (ElapsedSeconds :type Float%20%28double-precision%29) (TriggeredSeconds :type Float%20%28double-precision%29) (InputAction :type Input%20Action%20Object%20Reference :default "/Game/Gunslinger/Input/IA_Look.IA_Look"))
  (Pawn|Input|AddControllerYawInput (.x ActionValue))
  (Pawn|Input|AddControllerPitchInput (.y ActionValue))
  (Variables|Default|SetTurn%20Value (.x ActionValue))
  (|TurnInPlace (.x ActionValue) (.x ActionValue)))

(event EventBeginPlay
  (bind _returnvalue (Transformation|GetActorLocation))
  (Variables|Default|SetMovement%20Component (Variables|Character|GetCharacterMovement))
  (bind _asbp_gunslinger_player_controller (Utilities|Casting|CastToBP_GunslingerPlayerController (Pawn|GetController)))
  (Input|AddMappingContext (PlayerController|LocalPlayerSubsystems|GetEnhancedInputLocalPlayerSubsystem _asbp_gunslinger_player_controller) "/Game/Gunslinger/Input/IMC_Default.IMC_Default" 0 "(bIgnoreAllPressedKeysUntilRelease=True,bForceImmediately=False,bNotifyUserSettings=False)")
  (GameplayEffects|ApplyGameplayEffectToSelf :self (Variables|Default|GetAbilitySystemComponent) :GameplayEffectClass (Variables|Default|GetInitGameplayEffect))
  (bind _asplayer_controller (Utilities|Casting|CastToPlayerController (Pawn|GetController)))
  (Input|SetInputModeGameOnly _asplayer_controller false)
  (bind _returnvalue_2 (UserInterface|CreateWidget "/Game/Gunslinger/Blueprints/UI/HUD/WBP_Crosshair.WBP_Crosshair_C" _asplayer_controller))
  (UserInterface|Viewport|AddtoViewport _returnvalue_2 0)
  (Variables|Default|SetAmmo (.ReturnValue (Class|AbilitySystemComponent|GetGameplayAttributeValue (Variables|Default|GetAbilitySystemComponent) "(AttributeName=\"Armor\",Attribute=/Script/Gunslinger.RuneAttributeSet:Armor,AttributeOwner=\"/Script/CoreUObject.Class'/Script/Gunslinger.RuneAttributeSet'\")")))
  (bind _returnvalue_3 (UserInterface|CreateWidget "/Game/Gunslinger/Blueprints/UI/HUD/WBP_HUD.WBP_HUD_C" _asplayer_controller))
  (UserInterface|Viewport|AddtoViewport _returnvalue_3 0)
  (bind _returnvalue_4 (UserInterface|CreateWidget "/Game/Gunslinger/Blueprints/UI/HUD/WBP_FadeScreen.WBP_FadeScreen_C" _asplayer_controller))
  (UserInterface|Viewport|AddtoViewport _returnvalue_4 0)
  (bind _returnvalue_5 (UserInterface|CreateWidget "/Game/Gunslinger/Blueprints/UI/HUD/WBP_ScreenFlashRed.WBP_ScreenFlashRed_C" _asplayer_controller))
  (bind _output_get (Variables|Default|SetFlashRedWidget _returnvalue_5))
  (UserInterface|Viewport|AddtoViewport _output_get 0)
  (bind _newvalue (Ability|Tasks|WaitForAttributeChanged 0 "(AttributeName=\"CurrentHealth\",Attribute=/Script/Gunslinger.RuneAttributeSet:CurrentHealth,AttributeOwner=\"/Script/CoreUObject.Class'/Script/Gunslinger.RuneAttributeSet'\")")
    (:Changed
      (if (<= _newvalue 0.0)
        (Utilities|FlowControl|DoOnce false
          (:Completed
            (bind _returnvalue_6 (UserInterface|CreateWidget "/Game/Gunslinger/Blueprints/UI/HUD/WBP_DeathScreen.WBP_DeathScreen_C" _asplayer_controller))
            (UserInterface|Viewport|AddtoViewport _returnvalue_6 0)
            (Collision|SetCollisionEnabled (Variables|Default|GetCapsuleComponent) "NoCollision")
            (Components|Animation|PlayAnimation (Variables|Character|GetMesh) "/Game/Gunslinger/Animations/Ranger/AM_Death_Ranger.AM_Death_Ranger" false)
            (Class|UserWidget|PlayAnimationReverse _returnvalue_4 (Variables|/Game/Gunslinger/Blueprints/UI/HUD/WBP_FadeScreen.WBP_FadeScreen_C|GetFadeIn _returnvalue_4) 0.3 false)
            (Input|SetInputModeUIOnly (Game|GetPlayerController 0) 0 "LockAlways" false)
            (Audio|PlaySoundatLocation "/Game/Assets/HumanVocalizations/HumanFemaleB/Wavs/voice_female_b_death_08.voice_female_b_death_08" _returnvalue "0, 0, 0" 1.0 1.0 0.0 0 0 0 0)
            (Utilities|FlowControl|Delay 3.7)
            (Widget|SetVisibility _returnvalue_6 "Visible")
            (Variables|/Script/Engine.PlayerController|SetbShowMouseCursor (Game|GetPlayerController 0) true)
            (Game|SetGamePaused true)))
        (else
          (Default|PlayFlashAnim (Variables|Default|GetFlashRedWidget))
          (Audio|PlaySoundatLocation "/Game/Gunslinger/Sounds/Voice/SC_Hurt.SC_Hurt" _returnvalue "0, 0, 0" 1.0 1.0 0.0 0 0 0 0))))))

(event Collision|EventActorBeginOverlap
  (params (OtherActor :type Actor%20Object%20Reference))
  (bind _astrigger_volume (Utilities|Casting|CastToTriggerVolume OtherActor))
  (if (not (Collision|IsOverlappingActor (Variables|Character|GetMesh) _astrigger_volume :!class /Script/Engine.PrimitiveComponent))
    (Variables|Default|SetFootstepSound "/Game/Gunslinger/Sounds/Footsteps/SC_Footstep_Water.SC_Footstep_Water")))

(event Collision|EventActorEndOverlap
  (params (OtherActor :type Actor%20Object%20Reference))
  (Utilities|Casting|CastToTriggerVolume OtherActor)
  (Variables|Default|SetFootstepSound "/Game/Gunslinger/Sounds/Footsteps/SC_Footstep_Dirt.SC_Footstep_Dirt"))

(event Input|ActionEvents|InputActionOpenMainMenu
  (params (Key :type Key%20Structure :default "None"))
  (bind _returnvalue (Game|GetPlayerController 0))
  (bind _returnvalue_2 (Game|GetPlayerController 0))
  (:Pressed
    (bind _output_get (Variables|Default|SetPause (not (Variables|Default|GetPause))))
    (Game|SetGamePaused _output_get)
    (if _output_get
      (bind _returnvalue_3 (UserInterface|CreateWidget "/Game/Gunslinger/Blueprints/UI/Menu/WBP_Pause_Menu.WBP_Pause_Menu_C" _returnvalue_2))
      (UserInterface|Viewport|AddtoViewport _returnvalue_3 0)
      (Input|SetInputModeGameandUI _returnvalue _returnvalue_3 "DoNotLock" true false)
      (Variables|/Script/Engine.PlayerController|SetbShowMouseCursor _returnvalue true)
      (else
        (Widget|RemovefromParent _returnvalue_3)
        (Variables|/Script/Engine.PlayerController|SetbShowMouseCursor _returnvalue_2 false)
        (Input|SetInputModeGameOnly _returnvalue false)
        (Game|SetGamePaused false)))))

(fn ConstructionScript)