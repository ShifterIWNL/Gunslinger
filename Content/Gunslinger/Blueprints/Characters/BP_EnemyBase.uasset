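; Base enemy character for Gunslinger, built on the Gameplay Ability System, with name and health widgets.
; BeginPlay grants abilities via a gameplay effect and listens for attribute changes to update health; zero health triggers the defeat popup, death animation and death effect.
; Destruction may drop gold coins, and the first pawn sighting plays a growl.
; Helper functions expose combat ranges, patrol route and movement-speed tiers, and Attacked records the last attacker.
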(event OnSeePawn(PawnSensing)
  (params (Pawn :type Pawn%20Object%20Reference))
  (Utilities|FlowControl|DoOnce false
    (:Completed
      (Audio|PlaySoundatLocation "/Game/Assets/HumanVocalizations/HumanFemaleB/Wavs/voice_female_b_growl_groan_06.voice_female_b_growl_groan_06" (Transformation|GetActorLocation) "0, 0, 0" 0.7 0.6 0.0 0 0 0 0))))

(event Custom|Eliminated%20Widget
  (bind _returnvalue (UserInterface|CreateWidget "/Game/Gunslinger/Blueprints/UI/HUD/WBP_Defeated_Widget.WBP_Defeated_Widget_C" (Game|GetPlayerController 0)))
  (UserInterface|Animation|PlayAnimation _returnvalue (Variables|/Game/Gunslinger/Blueprints/UI/HUD/WBP_Defeated_Widget.WBP_Defeated_Widget_C|GetFade_Out _returnvalue) 0.0 1 "Forward" 1.0 false)
  (UserInterface|Viewport|AddtoViewport _returnvalue 0)
  (Utilities|FlowControl|Delay 1.3)
  (Widget|RemovefromParent _returnvalue))

(event Custom|Attacked
  (params (Attacker :type Actor%20Object%20Reference))
  (Variables|Default|SetLastAttacker Attacker))

(event EventDestroyed
  (CallFunction|DropLoot))

(event EventBeginPlay
  (bind _abilitysystemcomponent (Variables|Default|GetAbilitySystemComponent))
  (bind _returnvalue (Class|AbilitySystemComponent|GetGameplayAttributeValue _abilitysystemcomponent "(AttributeName=\"CurrentHealth\",Attribute=/Script/Gunslinger.RuneAttributeSet:CurrentHealth,AttributeOwner=\"/Script/CoreUObject.Class'/Script/Gunslinger.RuneAttributeSet'\")"))
  (bind _aswbp_enemy_name (Utilities|Casting|CastToWBP_EnemyName (UserInterface|GetWidget (Variables|Default|GetName))))
  (Default|UpdateName _aswbp_enemy_name (Variables|Default|GetEnemyName))
  (Utilities|FlowControl|Sequence
    (:then_0
      (GameplayEffects|ApplyGameplayEffectToSelf :self (Variables|Default|GetAbilitySystemComponent) :GameplayEffectClass "/Game/Gunslinger/Blueprints/Gameplay/Effects/GE_GrantAbilities.GE_GrantAbilities_C"))
    (:then_1
      (Ability|Tasks|WaitForAttributeChanged 0 "(AttributeName=\"CurrentHealth\",Attribute=/Script/Gunslinger.RuneAttributeSet:CurrentHealth,AttributeOwner=\"/Script/CoreUObject.Class'/Script/Gunslinger.RuneAttributeSet'\")"
        (:Changed
          (bind _aswbp_enemy_health_widget (Utilities|Casting|CastToWBP_EnemyHealthWidget (UserInterface|GetWidget (Variables|Default|GetHealth))))
          (Default|UpdateHealth _aswbp_enemy_health_widget _returnvalue (.ReturnValue (Class|AbilitySystemComponent|GetGameplayAttributeValue _abilitysystemcomponent "(AttributeName=\"MaxHealth\",Attribute=/Script/Gunslinger.RuneAttributeSet:MaxHealth,AttributeOwner=\"/Script/CoreUObject.Class'/Script/Gunslinger.RuneAttributeSet'\")")))
          (if (Math|Float|NearlyEqual(Float) _returnvalue 0.0 0.001)
            (CallFunction|EliminatedWidget)
            (Components|DestroyComponent (Variables|Default|GetHealth))
            (Components|DestroyComponent (Variables|Default|GetName))
            (Collision|SetCollisionResponsetoChannel (Variables|Character|GetMesh) "ECC_WorldStatic" "ECR_Ignore")
            (AI|ClearFocus (AI|GetAIController self))
            (Components|Animation|OverrideAnimationData (Variables|Character|GetMesh) "/Game/Gunslinger/Animations/Skeleton/AM_EnemyDeath.AM_EnemyDeath" false true 0.0 1.0)
            (GameplayEffects|ApplyGameplayEffectToSelf :self (Variables|Default|GetAbilitySystemComponent) :GameplayEffectClass "/Game/Gunslinger/Blueprints/Gameplay/Effects/GE_Death.GE_Death_C")))))))

(fn ConstructionScript)

(fn DropLoot
  (bind _self self)
  (bind _returnvalue (Transformation|GetActorTransform _self))
  (if (Math|Random|RandomBoolwithWeight 0.5)
    (bind _returnvalue_2 (Game|SpawnActorfromClass (.OutItem (Utilities|Array|Random (Utilities|Array|MakeArray "/Game/Gunslinger/Blueprints/Items/BP_GoldCoins.BP_GoldCoins_C" "/Game/Gunslinger/Blueprints/Items/BP_GoldCoins.BP_GoldCoins_C" "/Game/Gunslinger/Blueprints/Items/BP_GoldCoins.BP_GoldCoins_C"))) (Math|Transform|MakeTransform (Math|Vector|MakeVector (.x (.location _returnvalue)) (.y (.location _returnvalue)) (- (.z (.location _returnvalue)) 77.0)) (.rotation _returnvalue) (.scale _returnvalue)) "AdjustIfPossibleButAlwaysSpawn" "MultiplyWithRoot" 0 0))
    (if (== (Utilities|GetClass _returnvalue_2) "/Game/Gunslinger/Blueprints/Items/BP_GoldCoins.BP_GoldCoins_C")
      (Audio|PlaySoundatLocation "/Game/Gunslinger/Sounds/Coins/Coin_Drop.Coin_Drop" (Transformation|GetActorLocation) "0, 0, 0" 1.0 1.0 0.0 0 0 0 0))))

(fn GetIdealRange
  (return 8e+02 8e+02))

(fn GetPatrolRoute
  (return (Variables|AI|GetPatrolRoute)))

(fn SetMovementSpeed
  (params (Speed :type E_MovementSpeed%20Enum :default "NewEnumerator0"))
  (bind _output_get (Variables|/Script/Engine.CharacterMovementComponent|SetMaxWalkSpeed (Variables|Character|GetCharacterMovement) (Utilities|Select :Index Speed :NewEnumerator0 0.0 :NewEnumerator1 1e+02 :NewEnumerator2 2.5e+02 :NewEnumerator3 3.5e+02)))
  (return _output_get))