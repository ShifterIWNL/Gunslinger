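; BP_Chest is an interactable chest container that opens an inventory screen for the player.
; On interact, it passes its inventory component to the player controller's HUD and clears the Ranger's turn flags to prevent a rotation animation.
; When any overlap with its sphere ends, it removes every container inventory widget, without checking which actor left.
; Its Look At function returns an empty string.
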(event OnComponentEndOverlap(Sphere)
  (params (OverlappedComponent :type Primitive%20Component%20Object%20Reference) (OtherActor :type Actor%20Object%20Reference) (OtherComp :type Primitive%20Component%20Object%20Reference) (OtherBodyIndex :type Integer))
  (bind _foundwidgets (Widget|GetAllWidgetsOfClass "/Game/Gunslinger/Blueprints/UI/Inventory/WB_Container_Inventory.WB_Container_Inventory_C" false))
  (for _array_element _foundwidgets
    (Widget|RemovefromParent _array_element)))

(event EventInteractwith
  (params (Character :type BP%20Ranger%20Object%20Reference))
  (bind _asbp_gunslinger_player_controller (Utilities|Casting|CastToBP_GunslingerPlayerController (Game|GetPlayerController 0)))
  (Default|ShowContainer (Variables|/Game/Gunslinger/Blueprints/GameModes/Gunslinger/BP_GunslingerPlayerController.BP_GunslingerPlayerController_C|GetHUD _asbp_gunslinger_player_controller) (Variables|Default|GetAC_InventorySystem))
  ;[1 1 1] Prevent character rotation animation on interact
  (bind _asbp_ranger (Utilities|Casting|CastToBP_Ranger (Game|Player|GetPlayerPawn 0)))
  (Variables|/Game/Gunslinger/Blueprints/Characters/BP_Ranger.BP_Ranger_C|SetTurn%20Right _asbp_ranger false)
  (Variables|/Game/Gunslinger/Blueprints/Characters/BP_Ranger.BP_Ranger_C|SetTurn%20Left _asbp_ranger false))

(fn ConstructionScript)

(fn Lookat
  (return ""))