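; Patrol route actor for Skeleton AI that defines waypoints as the points of a spline.
; It tracks a current point index and direction, returning that point's world position on request.
; IncrementPatrolRoute steps the index along the spline and flips direction at either end, so the route runs back and forth rather than looping.
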(event Custom|IncrementPatrolRoute
  ;[1 1 1] if the index is positive it goes forward else it goes backwards
  (bind _output_get (Variables|Default|SetPatrolIndex (+ (Variables|Default|GetPatrolIndex) (Variables|Default|GetDirection))))
  (if (== _output_get (- (Spline|GetNumberOfSplinePoints (Variables|Default|GetPatrol%20Route)) 1))
    ;[1 1 1] patrols backwards up the spline
    (Variables|Default|SetDirection -1)
    (elif (== (Variables|Default|GetPatrolIndex) 0)
      (Variables|Default|SetDirection 1))))

(fn ConstructionScript)

(fn GetSplinePointasWorldPosition
  (return (Spline|GetLocationatSplinePoint (Variables|Default|GetPatrol%20Route) (Variables|Default|GetPatrolIndex) "World")))