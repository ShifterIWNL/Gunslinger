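; Gameplay ability that reloads the Ranger's weapon when its ammo is below a full load of twelve.
; It commits, plays the reload montage and applies GE_Reload to itself while the montage runs.
; Every montage exit, including interruption or cancellation, removes the effect, refills ammo, calls the Ranger's Reloaded notification and ends the ability.
; With full ammo or a failed cast, activation never reaches EndAbility.
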(event Ability|EventActivateAbility
  (bind _returnvalue (Ability|GetAbilitySystemComponentfromActorInfo))
  (bind _asbp_ranger (Utilities|Casting|CastToBP_Ranger (Ability|GetAvatarActorfromActorInfo)))
  (bind _output_get (Variables|Default|SetRanger _asbp_ranger))
  (if (< (Variables|/Game/Gunslinger/Blueprints/Characters/BP_Ranger.BP_Ranger_C|GetAmmo _output_get) 12.0)
    (Ability|CommitAbility)
    (|PlayMontageandWaitProxy "None" "/Game/Gunslinger/Animations/Ranger/AM_Reload_Ranger.AM_Reload_Ranger" 1.0 "None" true 1.0 0.0 false
      (:then
        (bind _returnvalue_2 (GameplayEffects|ApplyGameplayEffectToSelf :self _returnvalue :GameplayEffectClass "/Game/Gunslinger/Blueprints/Gameplay/Effects/GE_Reload.GE_Reload_C"))
        (Variables|Default|SetReloadHandle _returnvalue_2))
      (:OnCompleted
        (GameplayEffects|RemoveActiveGameplayEffect _returnvalue (Variables|Default|GetReloadHandle) -1 :!label _label)
        (Variables|/Game/Gunslinger/Blueprints/Characters/BP_Ranger.BP_Ranger_C|SetAmmo (Variables|Default|GetRanger) 12.0)
        (Default|CallReloaded (Variables|Default|GetRanger))
        (Ability|EndAbility))
      (:OnBlendOut
        (goto _label))
      (:OnInterrupted
        (goto _label))
      (:OnCancelled
        (goto _label)))))