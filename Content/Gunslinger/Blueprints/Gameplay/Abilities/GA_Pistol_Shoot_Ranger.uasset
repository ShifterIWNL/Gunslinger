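; Gameplay ability that fires the Ranger's pistol, spending ammo or playing an empty-trigger sound.
; A camera line trace finds the aim point, then a multi-trace from the weapon muzzle toward it gathers hits.
; Enemy head-component hits select critical over normal damage GameplayEffect, applied to the first hit actor.
; A fire montage then triggers weapon animation, shot and body-or-surface impact sounds, and ends the ability.
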(event Ability|EventActivateAbility
  (bind _returnvalue (Ability|GetAbilitySystemComponentfromActorInfo))
  (bind _asbp_ranger (Utilities|Casting|CastToBP_Ranger (Ability|GetAvatarActorfromActorInfo))
    (:then
      (bind _output_get (Variables|Default|SetRanger _asbp_ranger))
      (if (> (Variables|/Game/Gunslinger/Blueprints/Characters/BP_Ranger.BP_Ranger_C|GetAmmo (Variables|Default|GetRanger)) 0.0)
        (Ability|CommitAbility)
        (Math|Float|DecrementFloat (Variables|/Game/Gunslinger/Blueprints/Characters/BP_Ranger.BP_Ranger_C|GetAmmo (Variables|Default|GetRanger))
          (:%20%20
            (bind _outhit (Collision|LineTraceByChannel (Transformation|GetWorldLocation (Variables|/Script/Gunslinger.GunslingerCharacter|GetFollowCamera _output_get)) (+ (Transformation|GetWorldLocation (Variables|/Script/Gunslinger.GunslingerCharacter|GetFollowCamera _output_get)) (* (Math|Vector|GetForwardVector (Variables|/Script/Gunslinger.GunslingerCharacter|GetFollowCamera _output_get)) 1e+04)) "TraceTypeQuery1" false 0 "None"))
            (bind _outhits (Collision|MultiLineTraceByChannel (Transformation|GetSocketLocation (Variables|/Game/Gunslinger/Blueprints/Characters/BP_Ranger.BP_Ranger_C|GetWeapon (Variables|Default|GetRanger)) "Muzzle") (+ (Transformation|GetSocketLocation (Variables|/Game/Gunslinger/Blueprints/Characters/BP_Ranger.BP_Ranger_C|GetWeapon (Variables|Default|GetRanger)) "Muzzle") (* (- (Math|Vector|SelectVector (.Location (Collision|BreakHitResult _outhit)) (.TraceEnd (Collision|BreakHitResult _outhit)) (.bBlockingHit (Collision|BreakHitResult _outhit))) (Transformation|GetSocketLocation (Variables|/Game/Gunslinger/Blueprints/Characters/BP_Ranger.BP_Ranger_C|GetWeapon (Variables|Default|GetRanger)) "Muzzle")) 1.1)) "TraceTypeQuery2" false 0 "None"))
            (Variables|Default|SetFirstHit (Utilities|Array|Get(acopy) _outhits))
            (for _array_element _outhits
              (bind _asbp_enemy_base (Utilities|Casting|CastToBP_EnemyBase (.HitActor (Collision|BreakHitResult _array_element))))
              (Variables|Default|SetIsHeadshot (== (.HitComponent (Collision|BreakHitResult _array_element)) (Variables|/Game/Gunslinger/Blueprints/Characters/BP_EnemyBase.BP_EnemyBase_C|GetHead _asbp_enemy_base))))
            (bind _asgameplay_effect (Utilities|Casting|CastToGameplayEffectClass (Class|KismetMathLibrary|SelectClass "/Game/Gunslinger/Blueprints/Gameplay/Effects/GE_Damage_Critical_Pistol.GE_Damage_Critical_Pistol_C" "/Game/Gunslinger/Blueprints/Gameplay/Effects/GE_Damage_Pistol.GE_Damage_Pistol_C" (Variables|Default|GetIsHeadshot))))
            (GameplayEffects|ApplyGameplayEffectToTarget _returnvalue _asgameplay_effect (Ability|GetAbilitySystemComponent (.hitactor (Variables|Default|GetFirstHit))) 0.0 (GameplayEffects|MakeEffectContext _returnvalue))
            (Animation|Montage|PlayMontage (Variables|/Script/Engine.Character|GetMesh (Variables|Default|GetRanger)) "/Game/Gunslinger/Animations/Ranger/AM_Fire_Pistol.AM_Fire_Pistol" 1.7
              (:then
                (Audio|PlaySound2D "/Game/Assets/MilitaryWeapSilver/Sound/Pistol/Cues/PistolA_Fire_Cue.PistolA_Fire_Cue" 0.8 1.0 0.0 0 0)
                (Components|Animation|PlayAnimation (Variables|/Game/Gunslinger/Blueprints/Characters/BP_Ranger.BP_Ranger_C|GetWeapon (Variables|Default|GetRanger)) "/Game/Assets/MilitaryWeapSilver/Weapons/Animations/Fire_Pistol_W.Fire_Pistol_W" false)
                (if (Utilities|IsValid (Ability|GetAbilitySystemComponent (.hitactor (Variables|Default|GetFirstHit))))
                  (Audio|PlaySoundatLocation "/Game/Assets/MilitaryWeapSilver/Sound/Rifle/Cues/Rifle_ImpactBody_Cue.Rifle_ImpactBody_Cue" (.location (Variables|Default|GetFirstHit)) "0, 0, 0" 1.0 1.0 0.0 0 0 0 0)
                  (else
                    (Audio|PlaySoundatLocation "/Game/Assets/MilitaryWeapSilver/Sound/Rifle/Cues/Rifle_ImpactSurface_Cue.Rifle_ImpactSurface_Cue" (.location (Variables|Default|GetFirstHit)) "0, 0, 0" 1.0 1.0 0.0 0 0 0 0)))
                (Ability|EndAbility)))))
        (else
          (Audio|PlaySoundatLocation "/Game/Gunslinger/Sounds/Weapons/SC_TriggerEmpty.SC_TriggerEmpty" (Transformation|GetSocketLocation (Variables|/Game/Gunslinger/Blueprints/Characters/BP_Ranger.BP_Ranger_C|GetWeapon (Variables|Default|GetRanger)) "Muzzle") "0, 0, 0" 1.0 1.0 0.0 0 0 0 0))))
    (:CastFailed
      (Ability|EndAbility))))